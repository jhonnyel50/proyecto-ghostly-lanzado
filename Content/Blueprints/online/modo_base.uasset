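; Base game mode in the online folder that assigns spawn points to players by overriding ChoosePlayerStart.
; It counts the PlayerController actors in the world and returns the PlayerStart whose tag equals that number, so spawns follow the current player count.
; The Player argument is unused, no fallback handles a missing tag, and the event graph and construction script are empty.
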(fn `ChoosePlayerStart`
  (params (Player :type "Controller Object Reference"))
  (returns (ReturnValue :type "Actor Object Reference"))
  (bind _outactors (`GameplayStatics.GetAllActorsOfClass` "/Script/Engine.PlayerController"))
  (bind _outactors_2 (`GameplayStatics.GetAllActorsOfClass` "/Script/Engine.PlayerStart"))
  (for _array_element _outactors_2
    (if (== (`PlayerStart.PlayerStartTag` _array_element) (`KismetStringLibrary.Conv_StringToName` (`KismetStringLibrary.Conv_IntToString` (`KismetArrayLibrary.Array_Length` _outactors))))
      (return _array_element))))

(fn `UserConstructionScript`)